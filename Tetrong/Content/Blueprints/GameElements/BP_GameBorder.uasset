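; Border actor that builds the rectangular frame of the play screen from instanced cubes and spawns the first BP_BlockBase inside it.
; The construction script derives cube size from mesh bounds and scale, then fills an instanced mesh with two depth layers of side, top and bottom cubes sized by screen width and height.
; It also computes a spawn point near the top middle, which BeginPlay uses for the block.
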(event EventBeginPlay
  (Game|SpawnActorfromClass "/Game/Blueprints/GameElements/BP_BlockBase.BP_BlockBase_C" (Math|Transform|MakeTransform (Variables|Default|GetSpawn%20Point) "0, 0, 0" "1.000000,1.000000,1.000000") "Undefined" 0 0))

(event Collision|EventActorBeginOverlap
  (params (OtherActor :type Actor%20Object%20Reference)))

(event EventTick
  (params (DeltaSeconds :type Float%20%28single-precision%29)))

(fn ConstructionScript
  (bind _instancedcube (Variables|Default|GetInstancedCube))
  (bind _cube_scale (Variables|CubeProperties|GetCube%20Scale))
  (bind (_min _max) (Components|StaticMesh|GetLocalBounds _instancedcube))
  (bind _returnvalue (Math|Conversions|ToVector(Float) _cube_scale))
  (bind _returnvalue_2 (|((Max-Min)*Scale) _max _min _returnvalue))
  (Variables|CubeProperties|SetCube%20Width (.x _returnvalue_2))
  (Variables|CubeProperties|SetCube%20Depth (.y _returnvalue_2))
  (Variables|CubeProperties|SetCube%20Height (.z _returnvalue_2))
  (Development|PrintString (Utilities|String|Append "Construct" (Utilities|String|ToString(Float) _cube_scale)))
  (Private|SpawnScreen)
  (Private|SetupSpawnPoint))

(fn CreateVerticalBoundsforScreen
  (LocalVariables|SetVertical%20Offset (* (Variables|CubeProperties|GetCube%20Width) (- (Variables|ScreenDimensions|GetScreen%20Width) 1.0)))
  (for _index (range 0 (|(ScreenHeight-1) (Variables|ScreenDimensions|GetScreen%20Height)))
    (bind _output_get (LocalVariables|SetZPosition (* _index (Variables|CubeProperties|GetCube%20Height))))
    (bind _transform (Private|CreateTransform 0.0 0.0 _output_get))
    (Utilities|Array|Add (LocalVariables|GetBorder%20Cubes%20Transforms) _transform)
    (bind _transform_2 (Private|CreateTransform (Variables|CubeProperties|GetCube%20Depth) 0.0 (LocalVariables|GetZPosition)))
    (Utilities|Array|Add (LocalVariables|GetBorder%20Cubes%20Transforms) _transform_2)
    (bind _transform_3 (Private|CreateTransform 0.0 (LocalVariables|GetVertical%20Offset) (LocalVariables|GetZPosition)))
    (Utilities|Array|Add (LocalVariables|GetBorder%20Cubes%20Transforms) _transform_3)
    (bind _transform_4 (Private|CreateTransform (Variables|CubeProperties|GetCube%20Depth) (LocalVariables|GetVertical%20Offset) (LocalVariables|GetZPosition)))
    (Utilities|Array|Add (LocalVariables|GetBorder%20Cubes%20Transforms) _transform_4))
  (Components|InstancedStaticMesh|AddInstances (Variables|Default|GetInstancedCube) (LocalVariables|GetBorder%20Cubes%20Transforms) false false))

(fn CreateHorizontalBoundsforScreen
  (LocalVariables|SetHorizontal%20Offset (* (Variables|CubeProperties|GetCube%20Height) (- (Variables|ScreenDimensions|GetScreen%20Height) 1)))
  (for _index (range 1 (|(ScreenWidth-2) (Variables|ScreenDimensions|GetScreen%20Width)))
    (bind _output_get (LocalVariables|SetYPosition (* _index (Variables|CubeProperties|GetCube%20Height))))
    (bind _transform (Private|CreateTransform 0.0 _output_get 0.0))
    (Utilities|Array|Add (LocalVariables|GetBorder%20Cubes%20Transforms) _transform)
    (bind _transform_2 (Private|CreateTransform (Variables|CubeProperties|GetCube%20Depth) (LocalVariables|GetYPosition) 0.0))
    (Utilities|Array|Add (LocalVariables|GetBorder%20Cubes%20Transforms) _transform_2)
    (bind _transform_3 (Private|CreateTransform 0.0 (LocalVariables|GetYPosition) (LocalVariables|GetHorizontal%20Offset)))
    (Utilities|Array|Add (LocalVariables|GetBorder%20Cubes%20Transforms) _transform_3)
    (bind _transform_4 (Private|CreateTransform (Variables|CubeProperties|GetCube%20Depth) (LocalVariables|GetYPosition) (LocalVariables|GetHorizontal%20Offset)))
    (Utilities|Array|Add (LocalVariables|GetBorder%20Cubes%20Transforms) _transform_4))
  (Components|InstancedStaticMesh|AddInstances (Variables|Default|GetInstancedCube) (LocalVariables|GetBorder%20Cubes%20Transforms) false false))

(fn SpawnScreen
  (Private|CreateVerticalBoundsforScreen)
  (Private|CreateHorizontalBoundsforScreen))

(fn CreateTransform
  (params (X :type Float%20%28double-precision%29) (Y :type Float%20%28double-precision%29) (Z :type Float%20%28double-precision%29))
  (bind _cube_scale (Variables|CubeProperties|GetCube%20Scale))
  (Utilities|String|LogString (Utilities|String|Append "MakeTransform" (Utilities|String|ToString(Vector) (Math|Conversions|ToVector(Float) _cube_scale))))
  (return (Math|Transform|MakeTransform (Math|Vector|MakeVector X Y Z) "0.000000,90.000000,0.000000" (Math|Conversions|ToVector(Float) _cube_scale))))

(fn SetupSpawnPoint
  (bind _output_get (LocalVariables|SetRootLocation (Transformation|GetWorldLocation (Variables|Default|GetDefaultSceneRoot))))
  (Variables|Default|SetSpawn%20Point (Math|Vector|MakeVector (|SpawnPointX _output_get) (|SpawnPointY _output_get) (|SpawnPointZ _output_get))))